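; Player pawn that moves along its camera's forward and right vectors and interacts with nearby objects.
; Movement axes set actor location directly without sweep through AddMovement, whose speed and delta-time offset math appears unconnected.
; Capsule overlaps track one BI_Interactable actor via components tagged "interactable", toggling its prompt; the Interact input messages it.
; Any qualifying end overlap clears the tracked actor, even if another one left.
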(event OnComponentBeginOverlap(Capsule)
  (params (OverlappedComponent :type Primitive%20Component%20Object%20Reference) (OtherActor :type Actor%20Object%20Reference) (OtherComp :type Primitive%20Component%20Object%20Reference) (OtherBodyIndex :type Integer) (bFromSweep :type Boolean) (SweepResult :type Hit%20Result%20Structure%20%28by%20ref%29))
  (if (and (Utilities|DoesObjectImplementInterface OtherActor "/Game/Placeable/Interface/BI_Interactable.BI_Interactable_C") (Components|ComponentHasTag OtherComp "interactable"))
    (bind _interactableactor (Variables|Default|GetInteractableActor)
      (:then
        (Class|BIInteractable|EnableInteraction(Message) _interactableactor false))
      (:else
        _))
    (bind _output_get (Variables|Default|SetInteractableActor OtherActor))
    (Class|BIInteractable|EnableInteraction(Message) _output_get true)))

(event OnComponentEndOverlap(Capsule)
  (params (OverlappedComponent :type Primitive%20Component%20Object%20Reference) (OtherActor :type Actor%20Object%20Reference) (OtherComp :type Primitive%20Component%20Object%20Reference) (OtherBodyIndex :type Integer))
  (if (and (Utilities|DoesObjectImplementInterface OtherActor "/Game/Placeable/Interface/BI_Interactable.BI_Interactable_C") (Components|ComponentHasTag OtherComp "interactable"))
    (Class|BIInteractable|EnableInteraction(Message) (Variables|Default|GetInteractableActor) false)
    (Variables|Default|SetInteractableActor 0)))

(event Input|ActionEvents|InputActionInteract
  (params (Key :type Key%20Structure :default "None"))
  (:Pressed
    (bind _interactableactor (Variables|Default|GetInteractableActor)
      (:then
        (Class|BIInteractable|Interact(Message) _interactableactor))
      (:else))))

(event Input|AxisEvents|InputAxisMoveForward
  (params (AxisValue :type Float%20%28single-precision%29))
  (Transformation|SetActorLocation (Utilities|AddMovement AxisValue (Math|Vector|GetForwardVector (Variables|Default|GetCamera))) false false))

(event Input|AxisEvents|InputAxisMoveRight
  (params (AxisValue :type Float%20%28single-precision%29))
  (Transformation|SetActorLocation (Utilities|AddMovement AxisValue (Math|Vector|GetRightVector (Variables|Default|GetCamera))) false false))

(fn ConstructionScript)