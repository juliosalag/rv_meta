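; Placeable candle furniture that toggles its flames and light on interaction, or destroys a door when its Weapon condition is set.
; EnableInteraction shows or hides the interaction text.
; Interact destroys the referenced Door and the candle itself if Weapon is set.
; Otherwise it flips OnOff, switching four particle systems and setting visibility on the point light and main particle system.
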(event EventEnableInteraction
  (params (enable :type Boolean))
  (Rendering|SetVisibility (Variables|Default|GetInteractText) enable false))

(fn ConstructionScript
  (|CallParentFunction))

(fn Interact
  (if (Variables|Default|Getweapon)
    (Actor|DestroyActor (Variables|Default|Getdoor))
    (Actor|DestroyActor)
    (else
      (if (Variables|Default|GetbOnOff)
        (Components|Activation|Deactivate (Variables|Default|GetParticleSystem1))
        (Variables|Default|SetbOnOff false)
        (else
          (Components|Activation|Activate (Variables|Default|GetParticleSystem) true)
          (Variables|Default|SetbOnOff true)))
      (Rendering|SetVisibility (Variables|Default|GetPointLight) (Variables|Default|GetbOnOff) false)))
  (return true))